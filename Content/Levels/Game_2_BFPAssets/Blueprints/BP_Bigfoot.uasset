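; BP_Bigfoot is a flipbook Bigfoot that moves along a track spline while facing the photographer, acting as a timed target.
; BeginPlay finds BP_Track and picks random spline points, then NextPoint runs a Timeline that lerps between consecutive points, wrapping at a hardcoded index.
; After a fixed number of steps it calls Lose on the player's BP_Photographer.
; The won event stops the animation and movement.
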(event Custom|NextPoint
  (bind _track_ref (Variables|Default|GetTrack%20REF))
  (bind _spline (Variables|/Game/Levels/Game_1_BRAssets/Blueprints/BP_Track.BP_Track_C|GetSpline _track_ref))
  (if (== (Variables|Default|GetStepsTaken) 5)
    (bind _asbp_photographer (Utilities|Casting|CastToBP_Photographer (Game|Player|GetPlayerPawn 0)))
    (Default|Lose _asbp_photographer)
    (Audio|Components|Audio|Stop (Variables|Default|GetPaperFlipbook))
    (elif (== (Variables|Default|GetCurrent%20Point) 8)
      (Variables|Default|SetCurrent%20Point 0)
      (bind _bigfoot_move (Timeline|Timeline PlayFromStart)
        (:Update
          (Transformation|SetActorLocation (Math|Vector|Lerp(Vector) (Spline|GetLocationatSplinePoint _spline (Variables|Default|GetCurrent%20Point) "World") (Spline|GetLocationatSplinePoint _spline (+ (Variables|Default|GetCurrent%20Point) 1) "World") _bigfoot_move) false false)
          (bind _returnvalue (Actor|GetActorOfClass "/Game/Levels/Game_2_BFPAssets/Blueprints/BP_Photographer.BP_Photographer_C"))
          (Transformation|SetActorRotation (Math|Rotator|FindLookatRotation (Transformation|GetActorLocation) (Transformation|GetActorLocation _returnvalue))))
        (:Finished
          (Variables|Default|SetCurrent%20Point (+ (Variables|Default|GetCurrent%20Point) 1))
          (Variables|Default|SetStepsTaken (+ (Variables|Default|GetStepsTaken) 1))
          (CallFunction|NextPoint)))
      (else
        (Timeline|Timeline PlayFromStart)))))

(event Custom|won
  (bind _track_ref (Variables|Default|GetTrack%20REF))
  (bind _spline (Variables|/Game/Levels/Game_1_BRAssets/Blueprints/BP_Track.BP_Track_C|GetSpline _track_ref))
  (Audio|Components|Audio|Stop (Variables|Default|GetPaperFlipbook))
  (bind _bigfoot_move (Timeline|Timeline Stop)
    (:Update
      (Transformation|SetActorLocation (Math|Vector|Lerp(Vector) (Spline|GetLocationatSplinePoint _spline (Variables|Default|GetCurrent%20Point) "World") (Spline|GetLocationatSplinePoint _spline (+ (Variables|Default|GetCurrent%20Point) 1) "World") _bigfoot_move) false false)
      (bind _returnvalue (Actor|GetActorOfClass "/Game/Levels/Game_2_BFPAssets/Blueprints/BP_Photographer.BP_Photographer_C"))
      (Transformation|SetActorRotation (Math|Rotator|FindLookatRotation (Transformation|GetActorLocation) (Transformation|GetActorLocation _returnvalue))))
    (:Finished
      (Variables|Default|SetCurrent%20Point (+ (Variables|Default|GetCurrent%20Point) 1))
      (Variables|Default|SetStepsTaken (+ (Variables|Default|GetStepsTaken) 1))
      (CallFunction|NextPoint))))

(event EventBeginPlay
  (Variables|Default|SetStepsTaken 0)
  (bind _returnvalue (Actor|GetActorOfClass "/Game/Levels/Game_1_BRAssets/Blueprints/BP_Track.BP_Track_C"))
  (Variables|Default|SetTrack%20REF _returnvalue)
  (Variables|Default|SetCurrent%20Point (Math|Random|RandomIntegerinRange 0 (Spline|GetNumberOfSplinePoints (Variables|/Game/Levels/Game_1_BRAssets/Blueprints/BP_Track.BP_Track_C|GetSpline (Variables|Default|GetTrack%20REF)))))
  (Transformation|SetActorLocation (Spline|GetLocationatSplinePoint (Variables|/Game/Levels/Game_1_BRAssets/Blueprints/BP_Track.BP_Track_C|GetSpline (Variables|Default|GetTrack%20REF)) (Math|Random|RandomIntegerinRange 0 (Spline|GetNumberOfSplinePoints (Variables|/Game/Levels/Game_1_BRAssets/Blueprints/BP_Track.BP_Track_C|GetSpline (Variables|Default|GetTrack%20REF)))) "World") false false)
  (CallFunction|NextPoint))

(fn ConstructionScript)