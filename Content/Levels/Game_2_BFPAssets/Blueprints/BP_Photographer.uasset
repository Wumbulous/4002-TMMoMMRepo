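; Player-controlled photographer for a Bigfoot photo minigame, with a camera overlay widget and theme music.
; Left and right inputs turn it in 45-degree timeline steps, locking input during each turn.
; The cooldown-limited shutter wins if the Box overlaps BP_Bigfoot, notifying Bigfoot, cutting BP_Timer short and sliding in the winning photograph.
; A Lose event, not called here, stops the music and deducts a life through MMMM_GI.
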(event OnComponentBeginOverlap(Box)
  (params (OverlappedComponent :type Primitive%20Component%20Object%20Reference) (OtherActor :type Actor%20Object%20Reference) (OtherComp :type Primitive%20Component%20Object%20Reference) (OtherBodyIndex :type Integer) (bFromSweep :type Boolean) (SweepResult :type Hit%20Result%20Structure%20%28by%20ref%29))
  ;[1 1 1] Check Ovelap
  (Utilities|Casting|CastToBP_Bigfoot OtherActor)
  (Variables|Default|SetOverlapped true))

(event OnComponentEndOverlap(Box)
  (params (OverlappedComponent :type Primitive%20Component%20Object%20Reference) (OtherActor :type Actor%20Object%20Reference) (OtherComp :type Primitive%20Component%20Object%20Reference) (OtherBodyIndex :type Integer))
  ;[1 1 1] Check Ovelap
  (Utilities|Casting|CastToBP_Bigfoot OtherActor)
  (Variables|Default|SetOverlapped false))

(event Custom|Cool%20Down
  ;[1 1 1] Capture picture w/ cooldown
  (Variables|Default|SetCoolDown false))

(event Custom|Win
  (Utilities|FlowControl|Sequence
    (:then_0
      (Input|DisableInput (Game|GetPlayerController 0))
      (bind _returnvalue (Actor|GetActorOfClass "/Game/Levels/Game_2_BFPAssets/Blueprints/BP_Bigfoot.BP_Bigfoot_C"))
      (Default|Won _returnvalue)
      (bind _foundwidgets (Widget|GetAllWidgetsOfClass "/Game/Levels/Game_2_BFPAssets/UI/W_CameraOverlay.W_CameraOverlay_C" true))
      (Widget|RemovefromParent _foundwidgets)
      (bind _returnvalue_2 (Actor|GetActorOfClass "/Game/Blueprint/BP_Timer.BP_Timer_C"))
      (Variables|/Game/Blueprint/BP_Timer.BP_Timer_C|SetCutShort%20Time _returnvalue_2 2)
      (Default|CutShort _returnvalue_2))
    (:then_1
      (bind _newtrack_0 (Timeline|Timeline_0 Play)
        (:Update
          (Transformation|SetWorldLocation (Variables|Default|GetWinningPhotograph) (Math|Vector|Lerp(Vector) (Transformation|GetWorldLocation (Variables|Default|GetWinningPhotograph)) (Transformation|GetWorldLocation (Variables|Default|GetSpriteMovemTo)) _newtrack_0) false false))))))

(event Custom|Lose
  (Input|DisableInput (Game|GetPlayerController 0))
  (bind _asmmmm_gi (Utilities|Casting|CastToMMMM_GI (Game|GetGameInstance)))
  (Default|LostLife _asmmmm_gi)
  (Audio|Components|Audio|Stop (stale EventBeginPlay _returnvalue_2))
  (Audio|PlaySound2D "/Game/Levels/Game_2_BFPAssets/Audio/SFX/BFPD_FX_LOSE.BFPD_FX_LOSE" 1.0 1.0 0.0 0 0))

(event EventBeginPlay
  (Input|EnableInput (Game|GetPlayerController 0))
  (bind _returnvalue (UserInterface|CreateWidget "/Game/Levels/Game_2_BFPAssets/UI/W_CameraOverlay.W_CameraOverlay_C"))
  (UserInterface|Viewport|AddtoViewport _returnvalue 0)
  (bind _returnvalue_2 (Audio|SpawnSound2D "/Game/Levels/Game_2_BFPAssets/Audio/MX/BFPD_THEME.BFPD_THEME" 1.0 1.0 0.0 0)))

(event Input|ActionEvents|InputActionActionRight
  (params (Key :type Key%20Structure :default "None"))
  (:Pressed
    (Input|DisableInput (Game|GetPlayerController 0))
    (Variables|Default|SetCurrentRot (Transformation|GetActorRotation))
    (bind _newtrack_0 (Timeline|Timeline PlayFromStart)
      (:Update
        (Transformation|SetActorRotation (Math|Rotator|MakeRotator 0.0 0.0 (.yaw (Math|Rotator|Lerp(Rotator) (Variables|Default|GetCurrentRot) (Math|Rotator|MakeRotator 0.0 0.0 (+ (.Yaw (Math|Rotator|BreakRotator (Variables|Default|GetCurrentRot))) 45.0)) _newtrack_0)))))
      (:Finished
        (Input|EnableInput (Game|GetPlayerController 0))))))

(event Input|ActionEvents|InputActionActionLeft
  (params (Key :type Key%20Structure :default "None"))
  (:Pressed
    (Input|DisableInput (Game|GetPlayerController 0))
    (Variables|Default|SetCurrentRot (Transformation|GetActorRotation))
    (bind _leftrot (Timeline|LeftRot PlayFromStart)
      (:Update
        (Transformation|SetActorRotation (Math|Rotator|MakeRotator 0.0 0.0 (.yaw (Math|Rotator|Lerp(Rotator) (Variables|Default|GetCurrentRot) (Math|Rotator|MakeRotator 0.0 0.0 (- (.Yaw (Math|Rotator|BreakRotator (Variables|Default|GetCurrentRot))) 45.0)) _leftrot)))))
      (:Finished
        (Input|EnableInput (Game|GetPlayerController 0))))))

(event Input|ActionEvents|InputActionAction
  (params (Key :type Key%20Structure :default "None"))
  ;[1 1 1] Capture picture w/ cooldown
  (:Pressed
    (if (not (Variables|Default|GetCoolDown))
      (Variables|Default|SetCoolDown true)
      (Utilities|Time|SetTimerbyEvent (delegate Custom|Cool%20Down) (Variables|Default|GetCoolDownTime))
      (if (Variables|Default|GetOverlapped)
        (Audio|Components|Audio|Stop (stale EventBeginPlay _returnvalue_2))
        (Audio|PlaySound2D "/Game/Levels/Game_2_BFPAssets/Audio/SFX/BFPD_FX_WIN.BFPD_FX_WIN" 1.0 1.0 0.0 0 0)
        (CallFunction|Win)
        (else
          (Audio|PlaySound2D "/Game/Levels/Game_2_BFPAssets/Audio/SFX/BFPD_FX_CAMERA_FLASH.BFPD_FX_CAMERA_FLASH" 1.0 1.0 0.0 0 0))))))

(fn ConstructionScript)