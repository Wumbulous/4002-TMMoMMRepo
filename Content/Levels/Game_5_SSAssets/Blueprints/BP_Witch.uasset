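; Player witch for a minigame: it travels by projectile movement and switches between three spline-point lanes with left/right input.
; Timelines lerp mesh and capsule between points, locking input until each move finishes.
; Ouch drains health; at zero it stops movement, costs a life through MMMM_GI and shows the lose widget.
; Overlapping a TriggerVolume wins, turning the camera toward BP_Moon; both outcomes cut BP_Timer short.
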(event Custom|Lose
  (bind _returnvalue (Game|GetPlayerController 0))
  (bind _spline (Variables|Default|GetSpline))
  (bind _spline_2 (Variables|Default|GetSpline))
  (Audio|Components|Audio|Stop (stale EventBeginPlay _returnvalue))
  (Audio|PlaySound2D "/Game/Levels/Game_5_SSAssets/Audio/SFX/SS_FX_LOSE.SS_FX_LOSE" 1.0 1.0 0.0 0 0)
  (bind _asmmmm_gi (Utilities|Casting|CastToMMMM_GI (Game|GetGameInstance)))
  (Default|LostLife _asmmmm_gi)
  (bind _returnvalue_2 (Actor|GetActorOfClass "/Game/Blueprint/BP_Timer.BP_Timer_C"))
  (Variables|/Game/Blueprint/BP_Timer.BP_Timer_C|SetCutShort%20Time _returnvalue_2 3)
  (Default|CutShort _returnvalue_2)
  (Input|DisableInput (Game|GetPlayerController 0))
  (Components|Movement|StopMovementImmediately (Variables|Default|GetProjectileMovement))
  (Utilities|FlowControl|Sequence
    (:then_0
      (bind _newtrack_0 (Timeline|Timeline Stop)
        (:Update
          (Transformation|SetWorldLocation (Variables|Default|GetStaticMesh) (Math|Vector|Lerp(Vector) (Spline|GetLocationatSplinePoint _spline_2 (Variables|Default|GetCurrentPoint) "World") (Spline|GetLocationatSplinePoint _spline_2 (- (Variables|Default|GetCurrentPoint) 1) "World") _newtrack_0) false false))
        (:Finished
          (Variables|Default|SetCurrentPoint (Math|Integer|Clamp(Integer) (- (Variables|Default|GetCurrentPoint) 1) 0 2))
          (Input|EnableInput _returnvalue))))
    (:then_1
      (bind _newtrack_0_2 (Timeline|Timeline_0 Stop)
        (:Update
          (Transformation|SetWorldLocation (Variables|Default|GetStaticMesh) (Math|Vector|Lerp(Vector) (Spline|GetLocationatSplinePoint _spline (Variables|Default|GetCurrentPoint) "World") (Spline|GetLocationatSplinePoint _spline (+ (Variables|Default|GetCurrentPoint) 1) "World") _newtrack_0_2) false false))
        (:Finished
          (Variables|Default|SetCurrentPoint (Math|Integer|Clamp(Integer) (+ (Variables|Default|GetCurrentPoint) 1) 0 2))
          (Input|EnableInput _returnvalue))))))

(event Custom|Ouch
  (Variables|Default|SetHealth (- (Variables|Default|GetHealth) 1))
  (if (== (Variables|Default|GetHealth) 0)
    (CallFunction|Lose)
    (bind _returnvalue (UserInterface|CreateWidget "/Game/Levels/Game_5_SSAssets/W_WitchLose.W_WitchLose_C"))
    (Utilities|FlowControl|Delay 0.15)
    (UserInterface|Viewport|AddtoViewport _returnvalue 0)))

(event Collision|EventActorBeginOverlap
  (params (OtherActor :type Actor%20Object%20Reference))
  (bind _camera (Variables|Default|GetCamera))
  (Utilities|Casting|CastToTriggerVolume OtherActor)
  (Audio|PlaySound2D "/Game/Levels/Game_5_SSAssets/Audio/SFX/SS_FX_WIN.SS_FX_WIN" 1.0 1.0 0.0 0 0)
  (bind _returnvalue (Actor|GetActorOfClass "/Game/Blueprint/BP_Timer.BP_Timer_C"))
  (Variables|/Game/Blueprint/BP_Timer.BP_Timer_C|SetCutShort%20Time _returnvalue 3)
  (Default|CutShort _returnvalue)
  (bind _returnvalue_2 (Actor|GetActorOfClass "/Game/Levels/Game_5_SSAssets/Blueprints/BP_Moon.BP_Moon_C"))
  (bind _newtrack_0 (Timeline|Timeline_1 Play)
    (:Update
      (Transformation|SetWorldRotation (Variables|Default|GetCamera) (Math|Rotator|Lerp(Rotator) (Transformation|GetWorldRotation _camera) (Math|Rotator|FindLookatRotation (Transformation|GetWorldLocation _camera) (Transformation|GetActorLocation _returnvalue_2)) _newtrack_0) false false))
    (:Finished
      (Components|Movement|StopMovementImmediately (Variables|Default|GetProjectileMovement)))))

(event EventBeginPlay
  (Variables|Default|SetCurrentPoint 1)
  (Transformation|SetWorldLocation (Variables|Default|GetStaticMesh) (Spline|GetLocationatSplinePoint (Variables|Default|GetSpline) 1 "World") false false)
  (bind _returnvalue (Audio|SpawnSound2D "/Game/Levels/Game_5_SSAssets/Audio/MX/SS_THEME.SS_THEME" 1.0 1.0 0.0 0)))

(event Input|ActionEvents|InputActionActionRight
  (params (Key :type Key%20Structure :default "None"))
  (bind _returnvalue (Game|GetPlayerController 0))
  (bind _spline (Variables|Default|GetSpline))
  (:Pressed
    (Input|DisableInput _returnvalue)
    (bind _newtrack_0 (Timeline|Timeline PlayFromStart)
      (:Update
        (Transformation|SetWorldLocation (Variables|Default|GetStaticMesh) (Math|Vector|Lerp(Vector) (Spline|GetLocationatSplinePoint _spline (Variables|Default|GetCurrentPoint) "World") (Spline|GetLocationatSplinePoint _spline (- (Variables|Default|GetCurrentPoint) 1) "World") _newtrack_0) false false))
      (:Finished
        (Variables|Default|SetCurrentPoint (Math|Integer|Clamp(Integer) (- (Variables|Default|GetCurrentPoint) 1) 0 2))
        (Input|EnableInput _returnvalue)))))

(event Input|ActionEvents|InputActionActionLeft
  (params (Key :type Key%20Structure :default "None"))
  (bind _returnvalue (Game|GetPlayerController 0))
  (bind _spline (Variables|Default|GetSpline))
  (:Pressed
    (Input|DisableInput _returnvalue)
    (bind _newtrack_0 (Timeline|Timeline_0 PlayFromStart)
      (:Update
        (Transformation|SetWorldLocation (Variables|Default|GetStaticMesh) (Math|Vector|Lerp(Vector) (Spline|GetLocationatSplinePoint _spline (Variables|Default|GetCurrentPoint) "World") (Spline|GetLocationatSplinePoint _spline (+ (Variables|Default|GetCurrentPoint) 1) "World") _newtrack_0) false false))
      (:Finished
        (Variables|Default|SetCurrentPoint (Math|Integer|Clamp(Integer) (+ (Variables|Default|GetCurrentPoint) 1) 0 2))
        (Input|EnableInput _returnvalue)))))

(fn ConstructionScript)