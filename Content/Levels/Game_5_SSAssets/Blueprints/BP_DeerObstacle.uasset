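; Deer obstacle actor that darts along an offset from its start position when the player witch comes near.
; A Detect overlap with BP_Witch plays a leaves rustle and runs a timeline that lerps the actor from its BeginPlay location by TargetOffset, without sweeping.
; A separate Collision overlap with the witch only plays a 2D deer hit sound, with no damage or other effect applied here.
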(event OnComponentBeginOverlap(Collision)
  (params (OverlappedComponent :type Primitive%20Component%20Object%20Reference) (OtherActor :type Actor%20Object%20Reference) (OtherComp :type Primitive%20Component%20Object%20Reference) (OtherBodyIndex :type Integer) (bFromSweep :type Boolean) (SweepResult :type Hit%20Result%20Structure%20%28by%20ref%29))
  (Utilities|Casting|CastToBP_Witch OtherActor)
  (Audio|PlaySound2D "/Game/Levels/Game_5_SSAssets/Audio/SFX/SS_FX_DEER_HIT.SS_FX_DEER_HIT" 0.5 1.0 0.0 0 0))

(event OnComponentBeginOverlap(Detect)
  (params (OverlappedComponent :type Primitive%20Component%20Object%20Reference) (OtherActor :type Actor%20Object%20Reference) (OtherComp :type Primitive%20Component%20Object%20Reference) (OtherBodyIndex :type Integer) (bFromSweep :type Boolean) (SweepResult :type Hit%20Result%20Structure%20%28by%20ref%29))
  (bind _startpos (Variables|Default|GetStartPos))
  ;[1 1 1] When player enters detect, move by offset
  (Utilities|Casting|CastToBP_Witch OtherActor)
  (Audio|PlaySoundatLocation "/Game/Levels/Game_5_SSAssets/Audio/SFX/SS_FX_LEAVES_MOVE.SS_FX_LEAVES_MOVE" (Transformation|GetActorLocation) "0, 0, 0" 0.5 1.0 0.0 0 0 0 0)
  (bind _newtrack_0 (Timeline|Timeline Play)
    (:Update
      (Transformation|SetActorLocation (Math|Vector|Lerp(Vector) _startpos (+ _startpos (Variables|Default|GetTargetOffset)) _newtrack_0) false false))))

(event EventBeginPlay
  (Variables|Default|SetStartPos (Transformation|GetActorLocation)))

(fn ConstructionScript
  (|CallParentFunction))