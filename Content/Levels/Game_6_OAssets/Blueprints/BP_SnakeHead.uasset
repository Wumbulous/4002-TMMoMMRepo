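; Player-controlled snake head for a minigame where reaching BP_SnakeTail wins and hitting a BP_SnakeObstacle loses a life.
; Arrow-style inputs rotate it while blocking reversals, and a looping timer teleports it forward, spawning a body segment behind.
; Either collision swaps the face sprite, plays a sound, cuts BP_Timer short and halts movement and input.
; HangAround also costs a life through MMMM_GI if HungAround is still set.
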(event OnComponentBeginOverlap(Box)
  (params (OverlappedComponent :type Primitive%20Component%20Object%20Reference) (OtherActor :type Actor%20Object%20Reference) (OtherComp :type Primitive%20Component%20Object%20Reference) (OtherBodyIndex :type Integer) (bFromSweep :type Boolean) (SweepResult :type Hit%20Result%20Structure%20%28by%20ref%29))
  (Audio|Components|Audio|Stop (stale EventBeginPlay _returnvalue))
  (Utilities|Casting|CastToBP_SnakeObstacle OtherActor
    (:then
      (Rendering|Components|Sprite|SetSprite (Variables|Default|GetPaperSprite) "/Game/Levels/Game_6_OAssets/Textures/T_SnakeHeadSad_Sprite.T_SnakeHeadSad_Sprite")
      (bind _asmmmm_gi (Utilities|Casting|CastToMMMM_GI (Game|GetGameInstance)))
      (Default|LostLife _asmmmm_gi)
      (Audio|PlaySound2D "/Game/Levels/Game_6_OAssets/Audio/Sound/O_LOSE.O_LOSE" 1.0 1.0 0.0 0 0)
      (bind _returnvalue (Actor|GetActorOfClass "/Game/Blueprint/BP_Timer.BP_Timer_C"))
      (Default|CutShort _returnvalue))
    (:CastFailed
      (Utilities|Casting|CastToBP_SnakeTail OtherActor)
      (Rendering|Components|Sprite|SetSprite (Variables|Default|GetPaperSprite) "/Game/Levels/Game_6_OAssets/Textures/T_SnakeHeadHappy_Sprite.T_SnakeHeadHappy_Sprite")
      (Audio|PlaySound2D "/Game/Levels/Game_6_OAssets/Audio/Sound/O_WIN.O_WIN" 1.0 1.0 0.0 0 0)
      (bind _returnvalue_2 (Actor|GetActorOfClass "/Game/Blueprint/BP_Timer.BP_Timer_C"))
      (Variables|/Game/Blueprint/BP_Timer.BP_Timer_C|SetCutShort%20Time _returnvalue_2 2)
      (Default|CutShort _returnvalue_2)))
  (Utilities|Time|ClearandInvalidateTimerbyHandle (stale EventBeginPlay _returnvalue_2))
  (Input|DisableInput (Game|GetPlayerController 0))
  (Components|DestroyComponent (Variables|Default|GetBox))
  (Variables|Default|SetHungAround false))

(event Custom|HangAround
  (if (Variables|Default|GetHungAround)
    (bind _asmmmm_gi (Utilities|Casting|CastToMMMM_GI (Game|GetGameInstance)))
    (Default|LostLife _asmmmm_gi)))

(event Custom|MoveForward
  (Variables|Default|SetLast%20Place (Transformation|GetActorLocation))
  (Transformation|Teleport (+ (* (Transformation|GetActorForwardVector) "30.000000,30.000000,0.000000") (Transformation|GetActorLocation)) (Transformation|GetActorRotation))
  (Game|SpawnActorfromClass "/Game/Levels/Game_6_OAssets/Blueprints/BP_SnakeBody.BP_SnakeBody_C" (Math|Transform|MakeTransform (Variables|Default|GetLast%20Place) (Transformation|GetActorRotation) "1.000000,1.000000,1.000000") "Undefined" "MultiplyWithRoot" 0 0))

(event EventBeginPlay
  (bind _returnvalue (Audio|SpawnSound2D "/Game/Levels/Game_6_OAssets/Audio/Music/O_THEME.O_THEME" 1.0 1.0 0.0 0))
  (bind _returnvalue_2 (Utilities|Time|SetTimerbyEvent (delegate Custom|MoveForward) (Variables|Default|GetTime) true)))

(event Input|ActionEvents|InputActionActionUp
  (params (Key :type Key%20Structure :default "None"))
  (:Pressed
    (if (not (Variables|Default|GetFacingDown))
      (Variables|Default|SetFacing%20Left false)
      (Variables|Default|SetFacing%20Right false)
      (Variables|Default|SetFacing%20Up true)
      (Transformation|SetActorRotation "0, 0, 0"))))

(event Input|ActionEvents|InputActionActionDown
  (params (Key :type Key%20Structure :default "None"))
  (:Pressed
    (if (not (Variables|Default|GetFacing%20Up))
      (Variables|Default|SetFacing%20Left false)
      (Variables|Default|SetFacing%20Right false)
      (Variables|Default|SetFacingDown true)
      (Transformation|SetActorRotation "0.000000,180.000000,0.000000"))))

(event Input|ActionEvents|InputActionActionRight
  (params (Key :type Key%20Structure :default "None"))
  (:Pressed
    (if (not (Variables|Default|GetFacing%20Left))
      (Variables|Default|SetFacing%20Up false)
      (Variables|Default|SetFacingDown false)
      (Variables|Default|SetFacing%20Right true)
      (Transformation|SetActorRotation "0.000000,90.000000,0.000000"))))

(event Input|ActionEvents|InputActionActionLeft
  (params (Key :type Key%20Structure :default "None"))
  (:Pressed
    (if (not (Variables|Default|GetFacing%20Right))
      (Variables|Default|SetFacing%20Up false)
      (Variables|Default|SetFacingDown false)
      (Variables|Default|SetFacing%20Left true)
      (Transformation|SetActorRotation "0.000000,-90.000000,0.000000"))))

(fn ConstructionScript)