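; BP_UFO is the player pawn in a timed minigame where a UFO drops a pyramid top onto its base.
; Axis inputs move the pawn, and Action enables physics on PyramidTop to drop it.
; Staying on BP_PyramidBase for a short timer wins; hitting a TriggerVolume loses a life, with both signalling BP_Sphinx, swapping audio, disabling input and shortening BP_Timer.
; HangAround costs a life if HungAround is still set.
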(event OnComponentBeginOverlap(PyramidTop)
  (params (OverlappedComponent :type Primitive%20Component%20Object%20Reference) (OtherActor :type Actor%20Object%20Reference) (OtherComp :type Primitive%20Component%20Object%20Reference) (OtherBodyIndex :type Integer) (bFromSweep :type Boolean) (SweepResult :type Hit%20Result%20Structure%20%28by%20ref%29))
  (Utilities|Casting|CastToBP_PyramidBase OtherActor
    (:then
      (bind _returnvalue (Utilities|Time|SetTimerbyEvent (delegate Custom|Win) 1.0)))
    (:CastFailed
      (Utilities|Casting|CastToTriggerVolume OtherActor)
      (bind _asmmmm_gi (Utilities|Casting|CastToMMMM_GI (Game|GetGameInstance)))
      (Default|LostLife _asmmmm_gi)
      (Audio|Components|Audio|Stop (stale EventBeginPlay _returnvalue))
      (Audio|PlaySound2D "/Game/Levels/Game_4TCFEAssets/Audio/Sound/TCFE_FX_LOSE.TCFE_FX_LOSE" 1.0 1.0 0.0 0 0)
      (bind _returnvalue_2 (Actor|GetActorOfClass "/Game/Levels/Game_4TCFEAssets/BluePrints/BP_Sphinx.BP_Sphinx_C"))
      (Default|Lose _returnvalue_2)
      (Input|DisableInput (Game|GetPlayerController 0))
      (Variables|Default|SetHungAround false)
      (bind _returnvalue_3 (Actor|GetActorOfClass "/Game/Blueprint/BP_Timer.BP_Timer_C"))
      (Variables|/Game/Blueprint/BP_Timer.BP_Timer_C|SetCutShort%20Time _returnvalue_3 3)
      (Default|CutShort _returnvalue_3))))

(event OnComponentEndOverlap(PyramidTop)
  (params (OverlappedComponent :type Primitive%20Component%20Object%20Reference) (OtherActor :type Actor%20Object%20Reference) (OtherComp :type Primitive%20Component%20Object%20Reference) (OtherBodyIndex :type Integer))
  (Utilities|Casting|CastToBP_PyramidBase OtherActor)
  (Utilities|Time|ClearandInvalidateTimerbyHandle (stale OnComponentBeginOverlap(PyramidTop) _returnvalue)))

(event Custom|Win
  (Physics|SetSimulatePhysics (Variables|Default|GetPyramid%20Top) false)
  (Audio|Components|Audio|Stop (stale EventBeginPlay _returnvalue))
  (bind _outactors (Actor|GetAllActorsOfClass "/Game/Levels/Game_4TCFEAssets/BluePrints/BP_Sphinx.BP_Sphinx_C"))
  (Default|Win _outactors)
  (Audio|PlaySound2D "/Game/Levels/Game_4TCFEAssets/Audio/Sound/TCFE_FX_WIN.TCFE_FX_WIN" 1.0 1.0 0.0 0 0)
  (Input|DisableInput (Game|GetPlayerController 0))
  (Variables|Default|SetHungAround false)
  (bind _returnvalue (Actor|GetActorOfClass "/Game/Blueprint/BP_Timer.BP_Timer_C"))
  (Variables|/Game/Blueprint/BP_Timer.BP_Timer_C|SetCutShort%20Time _returnvalue 3)
  (Default|CutShort _returnvalue))

(event Custom|HangAround
  (if (Variables|Default|GetHungAround)
    (bind _asmmmm_gi (Utilities|Casting|CastToMMMM_GI (Game|GetGameInstance)))
    (Default|LostLife _asmmmm_gi)))

(event EventBeginPlay
  (bind _returnvalue (Audio|SpawnSound2D "/Game/Levels/Game_4TCFEAssets/Audio/Music/TCFE_THEME.TCFE_THEME" 1.0 1.0 0.0 0)))

(event Input|ActionEvents|InputActionAction
  (params (Key :type Key%20Structure :default "None"))
  (:Pressed
    (Physics|SetSimulatePhysics (Variables|Default|GetPyramid%20Top) true)))

(event Input|AxisEvents|InputAxisMoveHori
  (params (AxisValue :type Float%20%28single-precision%29))
  (Pawn|Input|AddMovementInput (Math|Vector|GetRightVector (Variables|Collision|GetCapsuleComponent)) AxisValue false))

(event Input|AxisEvents|InputAxisMoveVert
  (params (AxisValue :type Float%20%28single-precision%29))
  (Pawn|Input|AddMovementInput (Math|Vector|GetForwardVector (Variables|Collision|GetCapsuleComponent)) AxisValue false))

(fn ConstructionScript)