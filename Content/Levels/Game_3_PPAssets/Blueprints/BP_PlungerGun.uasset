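; BP_PlungerGun is a level actor that swings its aim across a set of targets, then launches a plunger projectile.
; BeginPlay starts Aim, which reshuffles the remaining Targets, turns toward the first with a timeline-driven rotation lerp, removes it and repeats.
; Once the list is empty, Fire plays a sound, destroys the plunger sprite and spawns BP_PlungerProjectile at the Arrow's transform, facing the last target aimed at.
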(event Custom|Fire
  (bind _arrow (Variables|Default|GetArrow))
  (Audio|PlaySound2D "/Game/Levels/Game_3_PPAssets/Audio/FX/PP_FX_PLUNGER.PP_FX_PLUNGER" 1.0 1.0 0.0 0 0)
  (Components|DestroyComponent (Variables|Default|GetPlunger))
  (Game|SpawnActorfromClass "/Game/Levels/Game_3_PPAssets/Blueprints/BP_PlungerProjectile.BP_PlungerProjectile_C" (Math|Transform|MakeTransform (Transformation|GetWorldLocation _arrow) (Transformation|GetWorldRotation _arrow) "1.000000,1.000000,1.000000") "Undefined" "MultiplyWithRoot" 0 0))

(event Custom|Aim
  (bind _targets (Variables|Default|GetTargets))
  (Variables|Default|SetGunRotation (Transformation|GetActorRotation))
  (Utilities|Array|Shuffle _targets)
  (if (Utilities|Array|IsEmpty _targets)
    (CallFunction|Fire)
    (else
      (bind _aimtime (Timeline|AimTimeline PlayFromStart)
        (:Update
          (Transformation|SetActorRotation (Math|Rotator|Lerp(Rotator) (Variables|Default|GetGunRotation) (Math|Rotator|FindLookatRotation (Transformation|GetActorLocation) (Transformation|GetActorLocation (Utilities|Array|Get(acopy) _targets))) _aimtime)))
        (:Finished
          (Utilities|Array|RemoveIndex _targets)
          (CallFunction|Aim))))))

(event EventBeginPlay
  (CallFunction|Aim))

(fn ConstructionScript)