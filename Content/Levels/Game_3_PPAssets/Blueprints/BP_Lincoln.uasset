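; BP_Lincoln is the player-controlled Lincoln actor for the PP minigame (Game 3).
; Left, right and up inputs play timelines on press and reverse on release, tilting or scaling the static mesh while locking out the other two actions.
; It starts the theme music on BeginPlay; Win and Lose swap it for a result sound and disable input.
; Lose also stops the timelines, shows the loss sprite and calls LostLife on MMMM_GI.
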(event Custom|Win
  (Audio|Components|Audio|Stop (stale EventBeginPlay _returnvalue))
  (Audio|PlaySound2D "/Game/Levels/Game_3_PPAssets/Audio/FX/PP_FX_WIN.PP_FX_WIN" 1.0 1.0 0.0 0 0)
  (Input|DisableInput (Game|GetPlayerController 0)))

(event Custom|Lose
  (Audio|Components|Audio|Stop (stale EventBeginPlay _returnvalue))
  (Audio|PlaySound2D "/Game/Levels/Game_3_PPAssets/Audio/FX/PP_FX_LOSE.PP_FX_LOSE" 1.0 1.0 0.0 0 0)
  (Input|DisableInput (Game|GetPlayerController 0))
  (Rendering|Components|Sprite|SetSprite (Variables|Default|GetPaperSprite) "/Game/Levels/Game_3_PPAssets/Textures/T_LincolnLoss_Sprite.T_LincolnLoss_Sprite")
  (bind _asmmmm_gi (Utilities|Casting|CastToMMMM_GI (Game|GetGameInstance)))
  (Default|LostLife _asmmmm_gi)
  (Utilities|FlowControl|Sequence
    (:then_0
      (bind _righttime (Timeline|RightTimeline Stop)
        (:Update
          (Transformation|SetWorldRotation (Variables|Default|GetStaticMesh) (Math|Rotator|Lerp(Rotator) "0, 0, 0" "0.000000,0.000000,45.000000" _righttime) false false))))
    (:then_1
      (bind _lefttime (Timeline|LeftTimeLine Stop)
        (:Update
          (Transformation|SetWorldRotation (Variables|Default|GetStaticMesh) (Math|Rotator|Lerp(Rotator) "0, 0, 0" "0.000000,0.000000,-45.000000" _lefttime) false false))))
    (:then_2
      (bind _uptime (Timeline|UpTimeLine Stop)
        (:Update
          (Transformation|SetRelativeScale3D (Variables|Default|GetStaticMesh) (Math|Vector|Lerp(Vector) (Variables|Default|GetIntScale) (Variables|Default|GetTarget%20Scale) _uptime)))))))

(event EventBeginPlay
  (Variables|Default|SetIntScale (Transformation|GetWorldScale (Variables|Default|GetStaticMesh)))
  (bind _returnvalue (Audio|SpawnSound2D "/Game/Levels/Game_3_PPAssets/Audio/MX/PP_THEME.PP_THEME" 1.0 1.0 0.0 0)))

(event Input|ActionEvents|InputActionActionUp
  (params (Key :type Key%20Structure :default "None"))
  (:Pressed
    (if (not (Variables|Default|GetUpUnavailable))
      (Variables|Default|SetLeftUnavailable true)
      (Variables|Default|SetRightUnavailable true)
      (bind _uptime (Timeline|UpTimeLine Play)
        (:Update
          (Transformation|SetRelativeScale3D (Variables|Default|GetStaticMesh) (Math|Vector|Lerp(Vector) (Variables|Default|GetIntScale) (Variables|Default|GetTarget%20Scale) _uptime))))))
  (:Released
    (if (not (Variables|Default|GetUpUnavailable))
      (Variables|Default|SetLeftUnavailable false)
      (Variables|Default|SetRightUnavailable false)
      (Timeline|UpTimeLine Reverse))))

(event Input|ActionEvents|InputActionActionLeft
  (params (Key :type Key%20Structure :default "None"))
  (:Pressed
    (if (not (Variables|Default|GetLeftUnavailable))
      (Variables|Default|SetUpUnavailable true)
      (Variables|Default|SetRightUnavailable true)
      (bind _lefttime (Timeline|LeftTimeLine Play)
        (:Update
          (Transformation|SetWorldRotation (Variables|Default|GetStaticMesh) (Math|Rotator|Lerp(Rotator) "0, 0, 0" "0.000000,0.000000,-45.000000" _lefttime) false false)))))
  (:Released
    (if (not (Variables|Default|GetLeftUnavailable))
      (Variables|Default|SetUpUnavailable false)
      (Variables|Default|SetRightUnavailable false)
      (Timeline|LeftTimeLine Reverse))))

(event Input|ActionEvents|InputActionActionRight
  (params (Key :type Key%20Structure :default "None"))
  (:Pressed
    (if (not (Variables|Default|GetRightUnavailable))
      (Variables|Default|SetUpUnavailable true)
      (Variables|Default|SetLeftUnavailable true)
      (bind _righttime (Timeline|RightTimeline Play)
        (:Update
          (Transformation|SetWorldRotation (Variables|Default|GetStaticMesh) (Math|Rotator|Lerp(Rotator) "0, 0, 0" "0.000000,0.000000,45.000000" _righttime) false false)))))
  (:Released
    (if (not (Variables|Default|GetRightUnavailable))
      (Variables|Default|SetUpUnavailable false)
      (Variables|Default|SetLeftUnavailable false)
      (Timeline|RightTimeline Reverse))))

(fn ConstructionScript)