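; BP_TitleSnake is a title-screen snake actor that moves in discrete steps along its facing direction.
; BeginPlay starts a looping timer at the MoveTimer interval, which fires MoveForward in place of per-frame Tick movement.
; Each step saves the current position in LastPlace, then teleports the actor a fixed distance forward without changing its rotation.
; Nothing in this graph reads LastPlace or steers the snake.
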(event Custom|MoveForward
  (Variables|Default|SetLast%20Place (Transformation|GetActorLocation))
  (Transformation|Teleport (+ (* (Transformation|GetActorForwardVector) "30.000000,30.000000,30.000000") (Transformation|GetActorLocation)) (Transformation|GetActorRotation)))

(event Collision|EventActorBeginOverlap
  (params (OtherActor :type Actor%20Object%20Reference))
  (|CallParentFunction OtherActor) ; This node is disabled and will not be called.\nDrag off pins to build functionality.
)

(event EventBeginPlay
  (|CallParentFunction)
  (Utilities|Time|SetTimerbyEvent (delegate Custom|MoveForward) (Variables|Default|GetMoveTimer) true))

(event EventTick
  (params (DeltaSeconds :type Float%20%28single-precision%29))
  (|CallParentFunction DeltaSeconds) ; This node is disabled and will not be called.\nDrag off pins to build functionality.
)

(fn ConstructionScript
  (|CallParentFunction))