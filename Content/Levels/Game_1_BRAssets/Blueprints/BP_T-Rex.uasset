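; Player-controlled T-Rex for the Battersaurus Rex minigame, which swings a bat at a meteor and handles the game's music and outcomes.
; The Action input triggers a swing with a timer-based cooldown, and a swing while overlapping BP_Meteor hits it and wins.
; Win and Lose swap flipbooks and audio and disable input.
; Lose, which is not called here, also notifies BP_Fire and deducts a life through MMMM_GI.
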(event Custom|Lose
  ;[1 1 1] Lose
  (Audio|Components|Audio|Stop (stale EventBeginPlay _returnvalue))
  (Audio|PlaySound2D "/Game/Levels/Game_1_BRAssets/Audio/Sound/Battersaurus_Rex_LOSE.Battersaurus_Rex_LOSE" 1.0 1.0 0.0 0 0)
  (Sprite|SetFlipbook (Variables|Default|GetT-Rex) "/Game/Levels/Game_1_BRAssets/Flipbooks/FB_Lose.FB_Lose")
  (bind _returnvalue (Actor|GetActorOfClass "/Game/Levels/Game_1_BRAssets/Blueprints/BP_Fire.BP_Fire_C"))
  (Default|Lose _returnvalue)
  (Utilities|Time|ClearTimerbyFunctionName 0 "Cool Down")
  (Input|DisableInput (Game|GetPlayerController 0))
  (bind _asmmmm_gi (Utilities|Casting|CastToMMMM_GI (Game|GetGameInstance)))
  (Default|LostLife _asmmmm_gi))

(event Custom|Win
  ;[1 1 1] Win
  (Audio|Components|Audio|Stop (stale EventBeginPlay _returnvalue))
  (Audio|PlaySound2D "/Game/Levels/Game_1_BRAssets/Audio/Sound/Battersaurus_Rex_WIN.Battersaurus_Rex_WIN" 1.0 1.0 0.0 0 0)
  (Utilities|Time|ClearTimerbyFunctionName 0 "Cool Down")
  (Input|DisableInput (Game|GetPlayerController 0))
  (Utilities|FlowControl|Delay 0.5)
  (Sprite|SetFlipbook (Variables|Default|GetT-Rex) "/Game/Levels/Game_1_BRAssets/Flipbooks/FB_Win.FB_Win"))

(event EventBeginPlay
  (bind _returnvalue (Audio|SpawnSound2D "/Game/Levels/Game_1_BRAssets/Audio/Music/Battersaurus_Rex_Theme.Battersaurus_Rex_Theme" 1.0 1.0 0.0 0)))

(event Collision|EventActorBeginOverlap
  (params (OtherActor :type Actor%20Object%20Reference))
  ;[1 1 1] Meteor Overlap Detect
  (Utilities|Casting|CastToBP_Meteor OtherActor)
  (Variables|Default|SetMeteorOverlap true))

(event Collision|EventActorEndOverlap
  (params (OtherActor :type Actor%20Object%20Reference))
  ;[1 1 1] Meteor Overlap Detect
  (Utilities|Casting|CastToBP_Meteor OtherActor)
  (Variables|Default|SetMeteorOverlap false))

(event Input|ActionEvents|InputActionAction
  (params (Key :type Key%20Structure :default "None"))
  ;[1 1 1] Cool Down + Hit
  (:Pressed
    (if (not (Variables|Default|GetOnCoolDown))
      (Sprite|SetFlipbook (Variables|Default|GetT-Rex) "/Game/Levels/Game_1_BRAssets/Flipbooks/FB_T-RexSwinging.FB_T-RexSwinging")
      (Variables|Default|SetOnCoolDown true)
      (Utilities|Time|SetTimerbyFunctionName 0 "Cool Down" (Variables|Default|GetCoolDownTimer))
      (if (Variables|Default|GetMeteorOverlap)
        (Audio|PlaySound2D "/Game/Levels/Game_1_BRAssets/Audio/Sound/Battersaurus_Rex_BAT_HIT.Battersaurus_Rex_BAT_HIT" 1.0 1.0 0.0 0 0)
        (bind _returnvalue (Actor|GetActorOfClass "/Game/Levels/Game_1_BRAssets/Blueprints/BP_Meteor.BP_Meteor_C"))
        (Default|BeenHit _returnvalue)
        (CallFunction|Win)
        (else
          (Audio|PlaySound2D "/Game/Levels/Game_1_BRAssets/Audio/Sound/Battersaurus_Rex_BAT_MISS.Battersaurus_Rex_BAT_MISS" 1.0 1.0 0.0 0 0))))))

(fn ConstructionScript)

(fn CoolDown
  (Variables|Default|SetOnCoolDown false)
  (Sprite|SetFlipbook (Variables|Default|GetT-Rex) "/Game/Levels/Game_1_BRAssets/Flipbooks/FB_T-Rex.FB_T-Rex"))