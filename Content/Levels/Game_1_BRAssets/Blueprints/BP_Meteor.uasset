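; BP_Meteor is a Paper2D meteor that travels along the BP_Track spline and makes BP_TRex lose if it reaches the end.
; On BeginPlay it finds the track and plays the MeteorMove timeline, which lerps distance along the spline to set its location.
; BeenHit stops the timeline, plays a non-looping hit flipbook and destroys the actor when that animation finishes.
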(event Custom|Move
  (bind _meteor_move (Timeline|MeteorMove Play)
    (:Update
      (Transformation|SetActorLocation (Spline|GetLocationatDistanceAlongSpline (Variables|/Game/Levels/Game_1_BRAssets/Blueprints/BP_Track.BP_Track_C|GetSpline (Variables|Default|GetTrackRef)) (Math|Float|Lerp 0.0 (Spline|GetSplineLength (Variables|/Game/Levels/Game_1_BRAssets/Blueprints/BP_Track.BP_Track_C|GetSpline (Variables|Default|GetTrackRef))) _meteor_move) "World") false false))
    (:Finished
      (bind _returnvalue (Actor|GetActorOfClass "/Game/Levels/Game_1_BRAssets/Blueprints/BP_T-Rex.BP_T-Rex_C"))
      (Default|Lose _returnvalue))))

(event Custom|BeenHit
  (bind _paperflipbook (Variables|Default|GetPaperFlipbook))
  (Sprite|SetFlipbook _paperflipbook "/Game/Levels/Game_1_BRAssets/Flipbooks/FB_MeteorBeenHit.FB_MeteorBeenHit")
  (Components|Timeline|SetLooping _paperflipbook false)
  (EventDispatchers|AssignOnFinishedPlaying _paperflipbook (delegate Custom|OnFinishedPlaying_Event))
  (bind _meteor_move (Timeline|MeteorMove Stop)
    (:Update
      (Transformation|SetActorLocation (Spline|GetLocationatDistanceAlongSpline (Variables|/Game/Levels/Game_1_BRAssets/Blueprints/BP_Track.BP_Track_C|GetSpline (Variables|Default|GetTrackRef)) (Math|Float|Lerp 0.0 (Spline|GetSplineLength (Variables|/Game/Levels/Game_1_BRAssets/Blueprints/BP_Track.BP_Track_C|GetSpline (Variables|Default|GetTrackRef))) _meteor_move) "World") false false))
    (:Finished
      (bind _returnvalue (Actor|GetActorOfClass "/Game/Levels/Game_1_BRAssets/Blueprints/BP_T-Rex.BP_T-Rex_C"))
      (Default|Lose _returnvalue))))

(event Custom|OnFinishedPlaying_Event
  (Actor|DestroyActor))

(event EventBeginPlay
  (bind _returnvalue (Actor|GetActorOfClass "/Game/Levels/Game_1_BRAssets/Blueprints/BP_Track.BP_Track_C"))
  (Variables|Default|SetTrackREF _returnvalue)
  (CallFunction|Move))

(fn ConstructionScript)