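; BP_Hand is the player-controlled hand in the Game 8 feather-plucking minigame, moved by axis input with a sprite swap on Action.
; Overlap events track when it is over a BP_Feather, and pressing Action destroys that feather and adds to the score.
; The sixth pluck swaps theme for win sound, cuts BP_Timer short, disables input and moves the CineCamera.
; HangAround costs a life through MMMM_GI while HungAround remains true.
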(event Custom|ScoreCheck
  (Variables|Default|SetScore (+ (Variables|Default|GetScore) 1))
  (if (== (Variables|Default|GetScore) 6)
    (Audio|Components|Audio|Stop (stale EventBeginPlay _returnvalue))
    (Audio|PlaySound2D "/Game/Levels/Game_8_BAMAssets/Audio/Sound/BAM_FX_WIN.BAM_FX_WIN" 1.0 1.0 0.0 0 0)
    (bind _returnvalue (Actor|GetActorOfClass "/Game/Blueprint/BP_Timer.BP_Timer_C"))
    (Variables|/Game/Blueprint/BP_Timer.BP_Timer_C|SetCutShort%20Time _returnvalue 2)
    (Default|CutShort _returnvalue)
    (Input|DisableInput (Game|GetPlayerController 0))
    (Variables|Default|SetHungAround false)
    (bind _returnvalue_2 (Actor|GetActorOfClass "/Script/CinematicCamera.CineCameraActor"))
    (Transformation|SetActorLocation _returnvalue_2 "-515.000000,1339.000000,15.000000" false false)))

(event Custom|HangAround
  (if (Variables|Default|GetHungAround)
    (bind _asmmmm_gi (Utilities|Casting|CastToMMMM_GI (Game|GetGameInstance)))
    (Default|LostLife _asmmmm_gi)))

(event EventBeginPlay
  (bind _returnvalue (Audio|SpawnSound2D "/Game/Levels/Game_8_BAMAssets/Audio/Music/BAM_THEME.BAM_THEME" 1.0 1.0 0.0 0)))

(event Collision|EventActorEndOverlap
  (params (OtherActor :type Actor%20Object%20Reference))
  (Utilities|Casting|CastToBP_Feather OtherActor)
  (Variables|Default|SetOverFeather false))

(event Collision|EventActorBeginOverlap
  (params (OtherActor :type Actor%20Object%20Reference))
  (bind _asbp_feather (Utilities|Casting|CastToBP_Feather OtherActor))
  (Variables|Default|SetOverFeather true))

(event Input|ActionEvents|InputActionAction
  (params (Key :type Key%20Structure :default "None"))
  (bind _papersprite (Variables|Default|GetPaperSprite))
  (:Pressed
    (Rendering|Components|Sprite|SetSprite _papersprite "/Game/Levels/Game_8_BAMAssets/Textures/T_Hand2_Sprite.T_Hand2_Sprite")
    (if (Variables|Default|GetOverFeather)
      (Utilities|IsValid (stale Collision|EventActorBeginOverlap _asbp_feather)
        (:Is%20Valid
          (Actor|DestroyActor (stale Collision|EventActorBeginOverlap _asbp_feather))
          (Audio|PlaySound2D "/Game/Levels/Game_8_BAMAssets/Audio/Sound/BAM_FX_PLUCK_L.BAM_FX_PLUCK_L" 1.0 1.0 0.0 0 0)
          (CallFunction|ScoreCheck)))))
  (:Released
    (Rendering|Components|Sprite|SetSprite _papersprite "/Game/Levels/Game_8_BAMAssets/Textures/T_Hand1_Sprite.T_Hand1_Sprite")))

(event Input|AxisEvents|InputAxisMoveVert
  (params (AxisValue :type Float%20%28single-precision%29))
  (Pawn|Input|AddMovementInput (Math|Vector|GetUpVector (Variables|Collision|GetCapsuleComponent)) AxisValue false))

(event Input|AxisEvents|InputAxisMoveHori
  (params (AxisValue :type Float%20%28single-precision%29))
  (Pawn|Input|AddMovementInput (Math|Vector|GetRightVector (Variables|Collision|GetCapsuleComponent)) AxisValue false))

(fn ConstructionScript)