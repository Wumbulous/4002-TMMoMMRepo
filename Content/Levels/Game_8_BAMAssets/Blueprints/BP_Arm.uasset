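; BP_Arm is a stretchable arm actor that visually reaches toward the hand of BP_Hand.
; Every Tick it looks up BP_Hand by class and rotates the whole actor to face the Hand component from its StaticMesh location.
; It then stretches the mesh's Z scale by the distance to the hand plus a small margin, keeping thickness fixed.
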(event EventTick
  (params (DeltaSeconds :type Float%20%28single-precision%29))
  (bind _staticmesh (Variables|Default|GetStaticMesh))
  (bind _returnvalue (Transformation|GetWorldLocation _staticmesh))
  (bind _returnvalue_2 (Actor|GetActorOfClass "/Game/Levels/Game_8_BAMAssets/Blueprints/BP_Hand.BP_Hand_C"))
  (Transformation|SetActorRotation (Math|Rotator|FindLookatRotation _returnvalue (Transformation|GetWorldLocation (Variables|/Game/Levels/Game_8_BAMAssets/Blueprints/BP_Hand.BP_Hand_C|GetHand _returnvalue_2))))
  (Transformation|SetWorldScale3D (Variables|Default|GetStaticMesh) (Math|Vector|MakeVector 0.17 0.17 (+ (/ (Math|Vector|Distance(Vector) _returnvalue (Transformation|GetWorldLocation (Variables|/Game/Levels/Game_8_BAMAssets/Blueprints/BP_Hand.BP_Hand_C|GetHand _returnvalue_2))) 1e+02) 0.05))))

(fn ConstructionScript)