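; BP_Cork is the cork in a giant-and-volcano minigame, a button-mash contest to push it down against a steady rise.
; A looping timer nudges it upward, while each externally triggered Mash moves it down twice as far.
; Its box overlapping BP_Volcano wins and stops the rise; hitting a TriggerVolume loses and costs a life via the GameInstance.
; Both outcomes disable input, remove visual components, cut BP_Timer short and destroy the giant's arms.
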(event OnComponentBeginOverlap(Box)
  (params (OverlappedComponent :type Primitive%20Component%20Object%20Reference) (OtherActor :type Actor%20Object%20Reference) (OtherComp :type Primitive%20Component%20Object%20Reference) (OtherBodyIndex :type Integer) (bFromSweep :type Boolean) (SweepResult :type Hit%20Result%20Structure%20%28by%20ref%29))
  (Utilities|Casting|CastToBP_Volcano OtherActor
    (:then
      (bind _asbp_giant (Utilities|Casting|CastToBP_Giant (Game|Player|GetPlayerPawn 0)))
      (Default|Win _asbp_giant)
      (Input|DisableInput _asbp_giant (Game|GetPlayerController 0))
      (Utilities|Time|ClearandInvalidateTimerbyHandle (stale EventBeginPlay _returnvalue))
      (Components|DestroyComponent (Variables|Default|GetHands)))
    (:CastFailed
      (Utilities|Casting|CastToTriggerVolume OtherActor)
      (bind _asbp_giant_2 (Utilities|Casting|CastToBP_Giant (Game|Player|GetPlayerPawn 0)))
      (Default|Lose _asbp_giant_2)
      (Input|DisableInput _asbp_giant_2 (Game|GetPlayerController 0))
      (bind _asmmmm_gi (Utilities|Casting|CastToMMMM_GI (Game|GetGameInstance)))
      (Default|LostLife _asmmmm_gi)
      (Components|DestroyComponent (Variables|Default|GetHands))))
  (bind _asbp_giant_3 (Utilities|Casting|CastToBP_Giant (Game|Player|GetPlayerPawn 0)))
  (Variables|/Game/Levels/Game_7_PAssets/Blueprints/BP_Giant.BP_Giant_C|SetHungAround _asbp_giant_3 false)
  (bind _returnvalue (Actor|GetActorOfClass "/Game/Blueprint/BP_Timer.BP_Timer_C"))
  (Default|CutShort _returnvalue)
  (bind _outactors (Actor|GetAllActorsOfClass "/Game/Levels/Game_7_PAssets/Blueprints/BP_GiantArms.BP_GiantArms_C"))
  (Actor|DestroyActor _outactors))

(event Custom|Mash
  (Transformation|SetActorLocation (- (Variables|Default|GetCurrentPos) "0.000000,0.000000,6.000000") false false)
  (Variables|Default|SetCurrentPos (- (Variables|Default|GetCurrentPos) "0.000000,0.000000,6.000000")))

(event Custom|PushUp
  (Transformation|SetActorLocation (+ (Variables|Default|GetCurrentPos) "0.000000,0.000000,3.000000") false false)
  (Variables|Default|SetCurrentPos (+ (Variables|Default|GetCurrentPos) "0.000000,0.000000,3.000000")))

(event EventBeginPlay
  (Variables|Default|SetCurrentPos (Transformation|GetActorLocation))
  (bind _returnvalue (Utilities|Time|SetTimerbyEvent (delegate Custom|PushUp) 0.1 true)))

(fn ConstructionScript)