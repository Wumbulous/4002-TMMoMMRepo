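; BP_Giant is the giant character of a microgame, driving its theme music, win/lose feedback and player input.
; It starts the theme on BeginPlay and forwards Action presses to BP_Cork's Mash.
; Win and Lose stop the music, play a sound, swap the sprite and cut BP_Timer short.
; HangAround deducts a life through the MMMM_GI game instance when HungAround is set.
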(event Custom|Hang%20Around
  (if (Variables|Default|GetHungAround)
    (bind _asmmmm_gi (Utilities|Casting|CastToMMMM_GI (Game|GetGameInstance)))
    (Default|LostLife _asmmmm_gi)))

(event Custom|Win
  (Audio|Components|Audio|Stop (stale EventBeginPlay _returnvalue))
  (Audio|PlaySound2D "/Game/Levels/Game_7_PAssets/Audio/FX/P_FX_WIN.P_FX_WIN" 1.0 1.0 0.0 0 0)
  (Rendering|Components|Sprite|SetSprite (Variables|Default|GetPaperSprite) "/Game/Levels/Game_7_PAssets/Textures/T_GiantWin_Sprite.T_GiantWin_Sprite")
  (bind _returnvalue (Actor|GetActorOfClass "/Game/Blueprint/BP_Timer.BP_Timer_C"))
  (Variables|/Game/Blueprint/BP_Timer.BP_Timer_C|SetCutShort%20Time _returnvalue 2)
  (Default|CutShort _returnvalue))

(event Custom|Lose
  (Audio|Components|Audio|Stop (stale EventBeginPlay _returnvalue))
  (Audio|PlaySound2D "/Game/Levels/Game_7_PAssets/Audio/FX/P_FX_LOSE.P_FX_LOSE" 1.0 1.0 0.0 0 0)
  (Rendering|Components|Sprite|SetSprite (Variables|Default|GetPaperSprite) "/Game/Levels/Game_7_PAssets/Textures/T_GiantLose_Sprite.T_GiantLose_Sprite")
  (bind _returnvalue (Actor|GetActorOfClass "/Game/Blueprint/BP_Timer.BP_Timer_C"))
  (Variables|/Game/Blueprint/BP_Timer.BP_Timer_C|SetCutShort%20Time _returnvalue 2)
  (Default|CutShort _returnvalue))

(event EventBeginPlay
  (bind _returnvalue (Audio|SpawnSound2D "/Game/Levels/Game_7_PAssets/Audio/MX/P_THEME.P_THEME" 1.0 1.0 0.0 0)))

(event Input|ActionEvents|InputActionAction
  (params (Key :type Key%20Structure :default "None"))
  (:Pressed
    (bind _returnvalue (Actor|GetActorOfClass "/Game/Levels/Game_7_PAssets/Blueprints/BP_Cork.BP_Cork_C"))
    (Utilities|IsValid _returnvalue
      (:Is%20Valid
        (Default|Mash _returnvalue)))))

(fn ConstructionScript)