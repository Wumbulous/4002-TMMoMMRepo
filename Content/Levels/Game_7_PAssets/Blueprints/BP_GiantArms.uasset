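; BP_GiantArms is a Paper2D sprite actor for giant arms that reach toward the BP_Cork actor in the level.
; Each tick it looks up the cork, rotates to face it, and stretches the sprite's X scale in proportion to the distance between them.
; When no cork exists it snaps to a fixed rotation.
; The Win event is an empty stub.
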(event Custom|Win)

(event EventTick
  (params (DeltaSeconds :type Float%20%28single-precision%29))
  (bind _papersprite (Variables|Default|GetPaperSprite))
  (bind _returnvalue (Transformation|GetWorldLocation _papersprite))
  (bind _returnvalue_2 (Actor|GetActorOfClass "/Game/Levels/Game_7_PAssets/Blueprints/BP_Cork.BP_Cork_C"))
  (Utilities|IsValid _returnvalue_2
    (:Is%20Valid
      (Transformation|SetActorRotation (Math|Rotator|FindLookatRotation _returnvalue (Transformation|GetActorLocation _returnvalue_2)))
      (Transformation|SetWorldScale3D _papersprite (Math|Vector|MakeVector (/ (Math|Vector|Distance(Vector) _returnvalue (Transformation|GetActorLocation _returnvalue_2)) 145.0) 2.0 2.0)))
    (:Is%20Not%20Valid
      (Transformation|SetActorRotation "90.000000,0.000000,0.000000"))))

(fn ConstructionScript)