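; BP_Timer is the round countdown for a series of minigames, starting a timer on BeginPlay that CutShort can replace with a shorter one.
; When it expires, it tries casting the player to Hand, Giant, Snake and UFO and calls HangAround on the match, which per a comment handles losing a life.
; It then reads Lives from MMMM_GI to open GameOver, or increments Score and opens Intermission, or End at the final score.
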(event Custom|TimerOver
  (bind _mygameins (Variables|Default|GetMyGameIns))
  (CallFunction|HandLifeCheck)
  (CallFunction|GiantLifeCheck)
  (CallFunction|SnakeLifeCheck)
  (CallFunction|UFOLifeCheck)
  (if (== (Variables|/Game/GameInstance/MMMM_GI.MMMM_GI_C|GetLives _mygameins) 0)
    (Game|OpenLevel(byName) "GameOver")
    (else
      (Variables|/Game/GameInstance/MMMM_GI.MMMM_GI_C|SetScore _mygameins (+ (Variables|/Game/GameInstance/MMMM_GI.MMMM_GI_C|GetScore _mygameins) 1))
      (if (== (Variables|/Game/GameInstance/MMMM_GI.MMMM_GI_C|GetScore _mygameins) 8)
        (Game|OpenLevel(byName) "End")
        (else
          (Game|OpenLevel(byName) "Intermission"))))))

(event Custom|CutShort
  ;[1 1 1] Comment
  (Utilities|Time|ClearandInvalidateTimerbyHandle (stale EventBeginPlay _returnvalue))
  (Utilities|Time|SetTimerbyEvent (delegate Custom|TimerOver) (Math|Conversions|ToFloat(Integer) (Variables|Default|GetCutShort%20Time))))

(event Custom|UFOLifeCheck
  ;[1 1 1] If player is allowed to be in a state in which they neither win nor lose "Hang Around" is called loosing a life
  (bind _asbp_ufo (Utilities|Casting|CastToBP_UFO (Game|GetPlayerCharacter 0)))
  (Default|HangAround _asbp_ufo))

(event Custom|SnakeLifeCheck
  ;[1 1 1] If player is allowed to be in a state in which they neither win nor lose "Hang Around" is called loosing a life
  (bind _asbp_snake_head (Utilities|Casting|CastToBP_SnakeHead (Game|Player|GetPlayerPawn 0)))
  (Default|HangAround _asbp_snake_head))

(event Custom|GiantLifeCheck
  ;[1 1 1] If player is allowed to be in a state in which they neither win nor lose "Hang Around" is called loosing a life
  (bind _asbp_giant (Utilities|Casting|CastToBP_Giant (Game|Player|GetPlayerPawn 0)))
  (Default|HangAround _asbp_giant))

(event Custom|HandLifeCheck
  ;[1 1 1] If player is allowed to be in a state in which they neither win nor lose "Hang Around" is called loosing a life
  (bind _asbp_hand (Utilities|Casting|CastToBP_Hand (Game|GetPlayerCharacter 0)))
  (Default|HangAround _asbp_hand))

(event EventBeginPlay
  (bind _asmmmm_gi (Utilities|Casting|CastToMMMM_GI (Game|GetGameInstance)))
  (Variables|Default|SetMyGameIns _asmmmm_gi)
  (bind _returnvalue (Utilities|Time|SetTimerbyEvent (delegate Custom|TimerOver) (Math|Conversions|ToFloat(Integer) (Variables|Default|GetTime)))))

(fn ConstructionScript)